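; BP_Door is a keyed door in Labwork904 that opens on Interact when the game mode's Keys value equals its KeyNumber.
; BeginPlay caches BP_GM_Labwork904; a match plays the DoorOpening timeline to slide the Cube upward, while a mismatch prints a wrong-key message.
; The construction script picks the Cube's material from MaterialArray by KeyNumber, so each door's look follows its required key.
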(event EventBeginPlay
  (bind _asbp_gm_labwork_904 (Utilities|Casting|CastToBP_GM_Labwork904 (Game|GetGameMode)))
  (Variables|Default|SetAs%20BP%20GM%20Labwork%20904 _asbp_gm_labwork_904))

(event EventInteract
  (if (== (Variables|/Game/Labwork904/Blueprints/BP_GM_Labwork904.BP_GM_Labwork904_C|GetKeys (Variables|Default|GetAs%20BP%20GM%20Labwork%20904)) (Variables|Default|GetKey%20Number))
    (bind _newtrack_0 (Timeline|Door%20Opening Play)
      (:Update
        (Transformation|SetRelativeLocation (Variables|Default|GetCube) (Math|Vector|Lerp(Vector) "0, 0, 0" "0.000000,0.000000,500.000000" _newtrack_0) false false)))
    (else
      (Development|PrintString "You don't have the correct key"))))

(fn ConstructionScript
  (Rendering|Material|SetMaterial (Variables|Default|GetCube) 0 (Utilities|Array|Get(acopy) (Variables|Default|GetMaterialArray) (Variables|Default|GetKey%20Number))))