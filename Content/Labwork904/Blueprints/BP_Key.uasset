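; BP_Key is a key pickup whose KeyNumber determines its material in the construction script.
; On BeginPlay it caches the BP_GM_Labwork904 game mode.
; Interact writes KeyNumber into the game mode's Keys value, replacing the previous one, prints an acquired message using the matching entry in Names, then destroys the actor.
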(event EventBeginPlay
  (bind _asbp_gm_labwork_904 (Utilities|Casting|CastToBP_GM_Labwork904 (Game|GetGameMode)))
  (Variables|Default|SetAs%20BP%20GM%20Labwork%20904 _asbp_gm_labwork_904))

(event Collision|EventActorBeginOverlap
  (params (OtherActor :type Actor%20Object%20Reference)))

(event EventTick
  (params (DeltaSeconds :type Float%20%28single-precision%29)))

(event EventInteract
  (bind _output_get (Variables|/Game/Labwork904/Blueprints/BP_GM_Labwork904.BP_GM_Labwork904_C|SetKeys (Variables|Default|GetAs%20BP%20GM%20Labwork%20904) (Variables|Default|GetKey%20Number)))
  (Development|PrintString (Utilities|String|Append "Key " (Utilities|Array|Get(acopy) (Variables|Default|GetNames) _output_get) "Acquired"))
  (Actor|DestroyActor))

(fn ConstructionScript
  (Rendering|Material|SetMaterial (Variables|Default|GetStaticMesh) 0 (Utilities|Array|Get(acopy) (Variables|Default|GetMaterialArray) (Variables|Default|GetKey%20Number))))