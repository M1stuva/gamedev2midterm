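; BP_MazeCell is a modular maze cell that procedurally builds its geometry in the construction script.
; It scales the floor from GridSize and adds cube-scaled wall meshes for each enabled side, plus an optional ceiling.
; Ceilinged cells with positive light intensity also get a point light.
; After a short delay at BeginPlay, it binds to BP_Manager's GameFinished dispatcher, recoloring that light when the event fires.
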(event Custom|E_GameFinished
  (params (Light%20Color :type Linear%20Color%20Structure))
  (Utilities|IsValid (Variables|Default|GetLightComponent)
    (:Is%20Valid
      (Rendering|Components|Light|SetLightColor (Variables|Default|GetLightComponent) Light%20Color true))))

(event EventBeginPlay
  (Utilities|FlowControl|Delay 0.2)
  (bind _returnvalue (Actor|GetActorOfClass "/Game/Labwork904/Blueprints/BP_Manager.BP_Manager_C"))
  (EventDispatchers|AssignGameFinished _returnvalue (delegate Custom|E_GameFinished)))

(event Collision|EventActorBeginOverlap
  (params (OtherActor :type Actor%20Object%20Reference)))

(event EventTick
  (params (DeltaSeconds :type Float%20%28single-precision%29)))

(fn ConstructionScript
  (bind _gridsize (Variables|Default|GetGridSize))
  (LocalVariables|SetWallLenght _gridsize)
  (LocalVariables|SetWallThickness (* _gridsize 0.1))
  (Transformation|SetRelativeScale3D (Variables|Default|GetFloor) (Utilities|SizetoCubeScale (Math|Vector|MakeVector (LocalVariables|GetWallLenght) (LocalVariables|GetWallLenght) (LocalVariables|GetWallThickness))))
  (if (Variables|Default|GetWestWall)
    (AddComponent|AddStaticMeshComponent false (Math|Transform|MakeTransform (Math|Vector|MakeVector 0.0 0.0 0.0) "0, 0, 0" (Utilities|SizetoCubeScale (Math|Vector|MakeVector (LocalVariables|GetWallLenght) (LocalVariables|GetWallThickness) (Variables|Default|GetWallHeight))))))
  (if (Variables|Default|GetSouthWall)
    (AddComponent|AddStaticMeshComponent false (Math|Transform|MakeTransform (Math|Vector|MakeVector 0.0 0.0 0.0) "0, 0, 0" (Utilities|SizetoCubeScale (Math|Vector|MakeVector (LocalVariables|GetWallThickness) (LocalVariables|GetWallLenght) (Variables|Default|GetWallHeight))))))
  (if (Variables|Default|GetEastWall)
    (AddComponent|AddStaticMeshComponent false (Math|Transform|MakeTransform (Math|Vector|MakeVector 0.0 (- (LocalVariables|GetWallLenght) (LocalVariables|GetWallThickness)) 0.0) "0, 0, 0" (Utilities|SizetoCubeScale (Math|Vector|MakeVector (LocalVariables|GetWallLenght) (LocalVariables|GetWallThickness) (Variables|Default|GetWallHeight))))))
  (if (Variables|Default|GetNorthWall)
    (AddComponent|AddStaticMeshComponent false (Math|Transform|MakeTransform (Math|Vector|MakeVector (- (LocalVariables|GetWallLenght) (LocalVariables|GetWallThickness)) 0.0 0.0) "0, 0, 0" (Utilities|SizetoCubeScale (Math|Vector|MakeVector (LocalVariables|GetWallThickness) (LocalVariables|GetWallLenght) (Variables|Default|GetWallHeight))))))
  (if (Variables|Default|GetCeiling)
    (AddComponent|AddStaticMeshComponent false (Math|Transform|MakeTransform (Math|Vector|MakeVector 0.0 0.0 (- (LocalVariables|GetWallLenght) (LocalVariables|GetWallThickness))) "0, 0, 0" (Utilities|SizetoCubeScale (Math|Vector|MakeVector (LocalVariables|GetWallLenght) (LocalVariables|GetWallLenght) (LocalVariables|GetWallThickness)))))
    (if (> (Variables|Default|GetLightIntensity) 0.0)
      (bind _returnvalue (AddComponent|AddPointLightComponent false (Math|Transform|MakeTransform (Math|Vector|MakeVector (* (LocalVariables|GetWallLenght) 0.5) (* (LocalVariables|GetWallLenght) 0.5) (* (Variables|Default|GetWallHeight) 0.75)) "0, 0, 0" "1.000000,1.000000,1.000000")))
      (Rendering|Components|Light|SetIntensity _returnvalue (Variables|Default|GetLightIntensity))
      (Rendering|Components|Light|SetLightColor _returnvalue (Variables|Default|GetNew%20Light%20Color) true)
      (Variables|Default|SetLightComponent _returnvalue))))