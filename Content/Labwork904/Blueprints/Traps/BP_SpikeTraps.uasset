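; BP_SpikeTraps is a spike trap that damages BP_Char904 characters through the player's DamageTake function.
; Overlapping the box while inactive waits a second, damages every character still inside, raises the spikes, and lowers them three seconds later.
; Characters entering while the trap is active take damage immediately.
; A timeline drives the spike mesh's height, playing forward to raise and in reverse to retract.
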(event OnComponentBeginOverlap(Box)
  (params (OverlappedComponent :type Primitive%20Component%20Object%20Reference) (OtherActor :type Actor%20Object%20Reference) (OtherComp :type Primitive%20Component%20Object%20Reference) (OtherBodyIndex :type Integer) (bFromSweep :type Boolean) (SweepResult :type Hit%20Result%20Structure%20%28by%20ref%29))
  (if (Variables|Default|GetIs%20Trap%20Activated)
    (bind _asbp_char_904 (Utilities|Casting|CastToBP_Char904 OtherActor))
    (bind _output_get (Variables|Default|SetAs%20BP%20Char%20904 _asbp_char_904))
    (Default|DamageTake _output_get (Variables|Default|GetDamage))
    (else
      (Utilities|FlowControl|Delay 1.0)
      (for _array_element (Collision|GetOverlappingActors (Variables|Default|GetBox) "/Game/Labwork904/Blueprints/BP_Char904.BP_Char904_C" :!class /Script/Engine.PrimitiveComponent)
        (bind _asbp_char_904_2 (Utilities|Casting|CastToBP_Char904 _array_element))
        (Default|DamageTake _asbp_char_904_2 (Variables|Default|GetDamage)))
      (Variables|Default|SetIs%20Trap%20Activated true)
      (CallFunction|SpikesUp)
      (Utilities|FlowControl|Delay 3.0)
      (CallFunction|SpikesDown)
      (Variables|Default|SetIs%20Trap%20Activated false))))

(event Custom|Spikes%20Down
  (bind _newtrack_0 (Timeline|SpikesTimeline ReverseFromEnd)
    (:Update
      (Transformation|SetRelativeLocation (Variables|Default|GetStaticMesh) (Math|Vector|MakeVector 0.0 0.0 (* _newtrack_0 5e+01)) false false))))

(event Custom|Spikes%20Up
  (bind _newtrack_0 (Timeline|SpikesTimeline PlayFromStart)
    (:Update
      (Transformation|SetRelativeLocation (Variables|Default|GetStaticMesh) (Math|Vector|MakeVector 0.0 0.0 (* _newtrack_0 5e+01)) false false))))

(event EventBeginPlay)

(event Collision|EventActorBeginOverlap
  (params (OtherActor :type Actor%20Object%20Reference)))

(event EventTick
  (params (DeltaSeconds :type Float%20%28single-precision%29)))

(fn ConstructionScript)