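; BP_Poisonous_Gas is a gas trap that deals repeated damage to a BP_Char904 character entering its box.
; Begin overlap stores the character and starts a looping one-second timer that calls DamageTake on it with the Damage value.
; End overlap waits three seconds before clearing that timer, so poisoning lingers after the character leaves.
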(event OnComponentBeginOverlap(Box)
  (params (OverlappedComponent :type Primitive%20Component%20Object%20Reference) (OtherActor :type Actor%20Object%20Reference) (OtherComp :type Primitive%20Component%20Object%20Reference) (OtherBodyIndex :type Integer) (bFromSweep :type Boolean) (SweepResult :type Hit%20Result%20Structure%20%28by%20ref%29))
  (bind _asbp_char_904 (Utilities|Casting|CastToBP_Char904 OtherActor))
  (Variables|Default|SetAs%20BP%20Char%20904 _asbp_char_904)
  (bind _returnvalue (Utilities|Time|SetTimerbyEvent (delegate Custom|Poison%20Player) 1.0 true))
  (Variables|Default|SetPoison%20Player%20Handle _returnvalue))

(event OnComponentEndOverlap(Box)
  (params (OverlappedComponent :type Primitive%20Component%20Object%20Reference) (OtherActor :type Actor%20Object%20Reference) (OtherComp :type Primitive%20Component%20Object%20Reference) (OtherBodyIndex :type Integer))
  (Utilities|Casting|CastToBP_Char904 OtherActor)
  (Utilities|FlowControl|Delay 3.0)
  (Utilities|Time|ClearandInvalidateTimerbyHandle (Variables|Default|GetPoison%20Player%20Handle)))

(event Custom|Poison%20Player
  (Default|DamageTake (Variables|Default|GetAs%20BP%20Char%20904) (Variables|Default|GetDamage)))

(fn ConstructionScript)