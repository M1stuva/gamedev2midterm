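; BP_SwingingAxe is a trap that swings a static mesh axe back and forth and damages the player character class on contact.
; From BeginPlay, SwingAxe uses a FlipFlop to alternate the Swing timeline between forward and reverse, re-entering it on Finished for an endless loop.
; The timeline track drives the mesh's relative pitch.
; Mesh overlaps with BP_Char904 call its DamageTake with the Damage value.
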(event OnComponentBeginOverlap(StaticMesh)
  (params (OverlappedComponent :type Primitive%20Component%20Object%20Reference) (OtherActor :type Actor%20Object%20Reference) (OtherComp :type Primitive%20Component%20Object%20Reference) (OtherBodyIndex :type Integer) (bFromSweep :type Boolean) (SweepResult :type Hit%20Result%20Structure%20%28by%20ref%29))
  (bind _asbp_char_904 (Utilities|Casting|CastToBP_Char904 OtherActor))
  (bind _output_get (Variables|Default|SetAs%20BP%20Char%20904 _asbp_char_904))
  (Default|DamageTake _output_get (Variables|Default|GetDamage)))

(event Custom|Swing%20Axe
  (Utilities|FlowControl|FlipFlop :!label _label
    (:A
      (bind _newtrack_0 (Timeline|Swing PlayFromStart)
        (:Update
          (Transformation|SetRelativeRotation (Variables|Default|GetStaticMesh) (Math|Rotator|MakeRotator 1.8e+02 (* _newtrack_0 6e+01) 9e+01) false false))
        (:Finished
          (goto _label))))
    (:B
      (Timeline|Swing ReverseFromEnd))))

(event EventBeginPlay
  (CallFunction|SwingAxe))

(event Collision|EventActorBeginOverlap
  (params (OtherActor :type Actor%20Object%20Reference)))

(event EventTick
  (params (DeltaSeconds :type Float%20%28single-precision%29)))

(fn ConstructionScript)